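; Player pawn that moves with Enhanced Input, drives a lantern and tracks draining life and lantern light values.
; BeginPlay adds the input mapping, shows the cursor, caches the BP_Lantern actor and creates the healthbar widget.
; While GamemodeActive, Tick moves the lantern, drains both values per frame without delta-time scaling, and caps only their maximum.
; IA_Move applies movement relative to control rotation.
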(event `self.ReceiveBeginPlay`
  (`|ExecutionSequence`
    (:`then_0`
      (bind _asplayer_controller (cast `PlayerController` (`self.GetController`)))
      (bind _returnvalue (pcsubsystem `EnhancedInputLocalPlayerSubsystem` _asplayer_controller))
      (`/Engine/EditorBlueprintResources/StandardMacros.IsValid` _returnvalue
        (:`Is Valid`
          (`EnhancedInputSubsystemInterface.AddMappingContext` _returnvalue "/Game/PlayerController/ActionMapping/IMC_Player.IMC_Player" 0 (struct))
          (set `PlayerController.bShowMouseCursor` true (`GameplayStatics.GetPlayerController` 0))
          (bind _returnvalue_2 (`GameplayStatics.GetActorOfClass` "/Game/PlayerController/BP_Lantern.BP_Lantern_C"))
          (set `self.LanternRef` _returnvalue_2))))
    (:`then_1`
      (bind _returnvalue_3 (`|CreateWidget` "/Game/PlayerController/WB_Healthbars.WB_Healthbars_C"))
      (`UserWidget.AddToViewport` _returnvalue_3 0))))

(event `self.ReceiveTick`
  (params (DeltaSeconds :type "Float (single-precision)"))
  (if (`self.GamemodeActive?`)
    (`/Game/PlayerController/BP_Lantern.MoveLantern` (`self.LanternRef`))
    (`|ExecutionSequence`
      (:`then_0`
        (set `self.LifeValue` (- (`self.LifeValue`) 1))
        (set `self.LanternLightValue` (- (`self.LanternLightValue`) 0.5)))
      (:`then_1`
        (if (> (`self.LanternLightValue`) 1000.0)
          (set `self.LanternLightValue` 1000.0)))
      (:`then_2`
        (if (> (`self.LifeValue`) 1000.0)
          (set `self.LifeValue` 1000.0))))))

(event `EnhancedInput|/Game/PlayerController/ActionMapping/Inputs/IA_Move`
  (params (ActionValue :type "Vector2D Structure") (ElapsedSeconds :type "Float (double-precision)") (TriggeredSeconds :type "Float (double-precision)") (InputAction :type "InputAction Object Reference" :default "/Game/PlayerController/ActionMapping/Inputs/IA_Move.IA_Move"))
  (bind (_returnvalue_roll _returnvalue_pitch _returnvalue_yaw) (`KismetMathLibrary.BreakRotator` (`self.GetControlRotation`)))
  (bind (_returnvalue_roll_2 _returnvalue_pitch_2 _returnvalue_yaw_2) (`KismetMathLibrary.BreakRotator` (`self.GetControlRotation`)))
  (:`Triggered`
    (`self.AddMovementInput` (`KismetMathLibrary.GetRightVector` (`KismetMathLibrary.MakeRotator` _returnvalue_roll_2 0.0 _returnvalue_yaw_2)) ActionValue_X)
    (`self.AddMovementInput` (`KismetMathLibrary.GetForwardVector` (`KismetMathLibrary.MakeRotator` 0.0 0.0 _returnvalue_yaw)) ActionValue_Y)))

(fn `UserConstructionScript`)